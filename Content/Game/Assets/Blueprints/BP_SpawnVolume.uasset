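; BP_SpawnVolume is a volume that keeps spawning InteractiveCubes at random points inside its Box component.
; On BeginPlay, a looping timer fires SpawnActor every half second, picking a random point within the box's scaled extent and skipping spawns that would collide.
; After each spawn attempt, it casts the game mode to ThirdPersonGameMode and calls IncreaseInteractiveCubes to update the cube counter, without checking whether the spawn succeeded.
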(event `self.ReceiveBeginPlay`
  ;[1 1 1] SpawningInRandomLocation
  (`KismetSystemLibrary.K2_SetTimerDelegate` (delegate `SpawnActor`) 0.5 true))

(event `SpawnActor`
  (bind _box (`self.Box`))
  ;[1 1 1] SpawningInRandomLocation
  (`|SpawnActorFromClass` "/Game/Game/Assets/Meshes/InteractiveCubes.InteractiveCubes_C" (`KismetMathLibrary.Conv_VectorToTransform` (`KismetMathLibrary.RandomPointInBoundingBox` (`SceneComponent.K2_GetComponentLocation` _box) (`BoxComponent.GetScaledBoxExtent` _box))) "DontSpawnIfColliding" "OverrideRootScale" null null)
  ;[1 1 1] ConnectingtToCounter
  (bind _asthird_person_game_mode (cast `/Game/ThirdPersonBP/Blueprints/ThirdPersonGameMode` (`GameplayStatics.GetGameMode`)))
  (`/Game/ThirdPersonBP/Blueprints/ThirdPersonGameMode.Increase_InteractiveCubes` _asthird_person_game_mode))

(fn `UserConstructionScript`)